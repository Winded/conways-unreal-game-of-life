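; Player pawn for a Game of Life simulation, handling camera control, simulation play/pause and cell editing.
; On BeginPlay it creates the GOLMenu widget and finds the LifeSimulator, whose click status it sets to activate or deactivate cells while paused.
; The camera toggles between a clamped, zoomable orbit around a lock point and free flight while the move button is held.
; SetLocked re-seats root and camera; Tick lerps the camera toward its target offset.
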(event EventTick
  (params (DeltaSeconds :type Float%20%28single-precision%29))
  (bind _cameraroot (Variables|Default|GetCameraRoot))
  (bind _camera (Variables|Default|GetCamera))
  (bind _moving (Variables|Utility|GetMoving))
  (bind _speed (Variables|GameOfLife|GetSpeed))
  (bind _cameraroot_2 (Variables|Default|GetCameraRoot))
  (bind _cameraroot_3 (Variables|Default|GetCameraRoot))
  (bind _returnvalue (Transformation|GetWorldRotation _cameraroot_3))
  (bind _returnvalue_2 (Transformation|GetWorldRotation _cameraroot))
  (bind _returnvalue_3 (Transformation|GetRelativeTransform _camera))
  (bind (_location _rotation) (Math|Transform|BreakTransform _returnvalue_3))
  (bind (_roll _pitch _yaw) (Math|Rotator|BreakRotator _returnvalue))
  (bind (_roll_2 _pitch_2 _yaw_2) (Math|Rotator|BreakRotator _returnvalue_2))
  (if (Variables|Utility|GetLocked)
    (Utilities|FlowControl|Sequence
      (:then_0
        (if _moving
          ;[1 1 1] Rotate camera by mouse delta (locked)
          (bind _asplayer_controller (Utilities|Casting|CastToPlayerController (Pawn|GetController)))
          (Transformation|SetWorldRotation _cameraroot_3 (Math|Rotator|MakeRotator 0.0 (Math|Float|Clamp(Float) (+ _pitch (.DeltaY (Class|PlayerController|GetInputMouseDelta _asplayer_controller))) (Variables|GameOfLife|GetMinimum%20Locked%20Pitch) (Variables|GameOfLife|GetMaximum%20Locked%20Pitch)) (+ _yaw (.DeltaX (Class|PlayerController|GetInputMouseDelta _asplayer_controller)))) false false)))
      (:then_1
        ;[1 1 1] Apply distance to target position
        (Variables|Utility|SetTarget%20Position (Math|Vector|MakeVector (* (Variables|GameOfLife|GetLock%20Distance) -1.0) 0.0 0.0)))
      (:then_2
        ;[1 1 1] Blend camera towards target position and rotaion
        (Transformation|SetRelativeLocationAndRotation _camera (Math|Vector|Lerp(Vector) _location (Variables|Utility|GetTarget%20Position) 0.25) (Math|Rotator|Lerp(Rotator) _rotation (Variables|Utility|GetTarget%20Rotation) 0.25 true) false false :!label _label)))
    (else
      (Utilities|FlowControl|Sequence
        (:then_0
          (if _moving
            (Utilities|FlowControl|Sequence
              (:then_0
                ;[1 1 1] Rotate camera by mouse delta (freely)
                (bind _asplayer_controller_2 (Utilities|Casting|CastToPlayerController (Pawn|GetController)))
                (Transformation|SetWorldRotation _cameraroot (Math|Rotator|MakeRotator _roll_2 (+ _pitch_2 (.DeltaY (Class|PlayerController|GetInputMouseDelta _asplayer_controller_2))) (+ _yaw_2 (.DeltaX (Class|PlayerController|GetInputMouseDelta _asplayer_controller_2)))) false false))
              (:then_1
                ;[1 1 1] Process free movement
                (Transformation|SetWorldLocation (Variables|Default|GetCameraRoot) (+ (+ (Transformation|GetWorldLocation _cameraroot_2) (* (Math|Vector|GetForwardVector _cameraroot_2) (* _speed (Variables|Utility|GetVertical%20Movement)))) (* (Math|Vector|GetRightVector _cameraroot_2) (* _speed (Variables|Utility|GetHorizontal%20Movement)))) false false)))))
        (:then_1
          (goto _label))))))

(event EventBeginPlay
  ;[1 1 1] Create user interface
  (bind _returnvalue (UserInterface|CreateWidget "/Game/Blueprints/GUI/GOLMenu.GOLMenu_C"))
  (bind _output_get (Variables|UI|SetMenu _returnvalue))
  (UserInterface|Viewport|AddtoViewport _output_get 0)
  ;[1 1 1] Find a life
  (bind _outactors (Actor|GetAllActorsOfClass "/Game/Blueprints/LifeSimulator.LifeSimulator_C"))
  (Variables|Utility|SetLife%20Simulator (Utilities|Array|Get(acopy) _outactors)))

(event Input|ActionEvents|InputActionDeactivateCell
  (params (Key :type Key%20Structure :default "AnyKey"))
  (bind _life_simulator (Variables|Utility|GetLife%20Simulator))
  ;[1 1 1] Cell activation/deactivation
  (:Pressed
    (if (not (Variables|/Game/Blueprints/LifeSimulator.LifeSimulator_C|GetSimulating _life_simulator))
      (Variables|/Game/Blueprints/LifeSimulator.LifeSimulator_C|SetClickStatus _life_simulator "NewEnumerator2")))
  (:Released
    (Variables|/Game/Blueprints/LifeSimulator.LifeSimulator_C|SetClickStatus _life_simulator "NewEnumerator0")))

(event Input|ActionEvents|InputActionMoveCameraFurther
  (params (Key :type Key%20Structure :default "AnyKey"))
  ;[1 1 1] Zoom locked camera in and out
  (:Pressed
    (if (Variables|Utility|GetLocked)
      (Variables|GameOfLife|SetLock%20Distance (Math|Float|Clamp(Float) (+ (Variables|GameOfLife|GetLock%20Distance) (Variables|GameOfLife|GetZoom%20Interval)) (Variables|GameOfLife|GetMinimum%20Distance) (Variables|GameOfLife|GetMaximum%20Distance))))))

(event Input|ActionEvents|InputActionMoveCameraCloser
  (params (Key :type Key%20Structure :default "AnyKey"))
  ;[1 1 1] Zoom locked camera in and out
  (:Pressed
    (if (Variables|Utility|GetLocked)
      (Variables|GameOfLife|SetLock%20Distance (Math|Float|Clamp(Float) (- (Variables|GameOfLife|GetLock%20Distance) (Variables|GameOfLife|GetZoom%20Interval)) (Variables|GameOfLife|GetMinimum%20Distance) (Variables|GameOfLife|GetMaximum%20Distance))))))

(event Input|ActionEvents|InputActionToggleSimulation
  (params (Key :type Key%20Structure :default "AnyKey"))
  (bind _life_simulator (Variables|Utility|GetLife%20Simulator))
  ;[1 1 1] Play/Pause simulation
  (:Pressed
    (Variables|/Game/Blueprints/LifeSimulator.LifeSimulator_C|SetSimulating _life_simulator (not (Variables|/Game/Blueprints/LifeSimulator.LifeSimulator_C|GetSimulating _life_simulator)))))

(event Input|ActionEvents|InputActionChangeCameraMode
  (params (Key :type Key%20Structure :default "AnyKey"))
  ;[1 1 1] Toggle camera mode
  (:Pressed
    (CallFunction|SetLocked (not (CallFunction|IsLocked)))))

(event Input|ActionEvents|InputActionMoveForward
  (params (Key :type Key%20Structure :default "AnyKey"))
  ;[1 1 1] Process free movement key events
  (:Pressed
    (Variables|Utility|SetVertical%20Movement 1.0))
  (:Released
    (Variables|Utility|SetVertical%20Movement 0.0)))

(event Input|ActionEvents|InputActionMoveRight
  (params (Key :type Key%20Structure :default "AnyKey"))
  ;[1 1 1] Process free movement key events
  (:Pressed
    (Variables|Utility|SetHorizontal%20Movement 1.0))
  (:Released
    (Variables|Utility|SetHorizontal%20Movement 0.0)))

(event Input|ActionEvents|InputActionMoveBackward
  (params (Key :type Key%20Structure :default "AnyKey"))
  ;[1 1 1] Process free movement key events
  (:Pressed
    (Variables|Utility|SetVertical%20Movement -1.0))
  (:Released
    (Variables|Utility|SetVertical%20Movement 0.0)))

(event Input|ActionEvents|InputActionMoveLeft
  (params (Key :type Key%20Structure :default "AnyKey"))
  ;[1 1 1] Process free movement key events
  (:Pressed
    (Variables|Utility|SetHorizontal%20Movement -1.0))
  (:Released
    (Variables|Utility|SetHorizontal%20Movement 0.0)))

(event Input|ActionEvents|InputActionMoveCamera
  (params (Key :type Key%20Structure :default "AnyKey"))
  (bind _returnvalue (Pawn|GetController))
  ;[1 1 1] Toggle movement
  (:Pressed
    (bind _asplayer_controller (Utilities|Casting|CastToPlayerController _returnvalue))
    (Variables|/Script/Engine.PlayerController|SetbShowMouseCursor _asplayer_controller false)
    (Variables|Utility|SetMoving true))
  (:Released
    (bind _asplayer_controller_2 (Utilities|Casting|CastToPlayerController _returnvalue))
    (Variables|/Script/Engine.PlayerController|SetbShowMouseCursor _asplayer_controller_2 true)
    (Variables|Utility|SetMoving false)))

(event Input|ActionEvents|InputActionActivateCell
  (params (Key :type Key%20Structure :default "AnyKey"))
  (bind _life_simulator (Variables|Utility|GetLife%20Simulator))
  ;[1 1 1] Cell activation/deactivation
  (:Pressed
    (if (not (Variables|/Game/Blueprints/LifeSimulator.LifeSimulator_C|GetSimulating _life_simulator))
      (Variables|/Game/Blueprints/LifeSimulator.LifeSimulator_C|SetClickStatus _life_simulator "NewEnumerator1")))
  (:Released
    (Variables|/Game/Blueprints/LifeSimulator.LifeSimulator_C|SetClickStatus _life_simulator "NewEnumerator0")))

(fn ConstructionScript)

(fn SetLocked
  (params (Locked :type Boolean))
  (bind _camera (Variables|Default|GetCamera))
  (bind _cameraroot (Variables|Default|GetCameraRoot))
  (bind _camera_2 (Variables|Default|GetCamera))
  (bind _cameraroot_2 (Variables|Default|GetCameraRoot))
  (LocalVariables|SetCamPos (Transformation|GetWorldLocation _camera))
  (LocalVariables|SetCamRot (Transformation|GetWorldRotation _camera))
  (if Locked
    (Transformation|SetWorldLocation _cameraroot (Variables|GameOfLife|GetLock%20Point) false false)
    (Transformation|SetWorldRotation _cameraroot (Variables|GameOfLife|GetInitial%20Rotation) false false)
    (Transformation|SetWorldLocation _camera_2 (LocalVariables|GetCamPos) false false)
    (Transformation|SetWorldRotation _camera_2 (LocalVariables|GetCamRot) false false)
    (else
      (Transformation|SetRelativeLocationAndRotation (Variables|Default|GetCamera) "0, 0, 0" "0, 0, 0" false false)
      (Transformation|SetWorldLocation _cameraroot_2 (LocalVariables|GetCamPos) false false)
      (Transformation|SetWorldRotation _cameraroot_2 (LocalVariables|GetCamRot) false false)))
  (Variables|Utility|SetLocked Locked))

(fn IsLocked
  (return (Variables|Utility|GetLocked)))