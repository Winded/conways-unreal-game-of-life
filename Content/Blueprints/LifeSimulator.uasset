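; Actor that runs a Conway's Game of Life grid, spawning a LifeCell actor for each position at BeginPlay.
; LifeSimulatorCore holds the grid state; while simulating, it cycles at a timed interval and every cell refreshes its material.
; While paused, Tick traces under the cursor and sets the hit cell alive or dead according to the click status, then updates its material.
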(event EventBeginPlay
  (bind _size (Variables|LifeSimulator|GetSize))
  ;[1 1 1] Generate cell grid
  (Class|LifeSimulatorCore|GenerateGrid (Variables|Default|GetLifeSimulatorCore) _size)
  (for _index (range 1 _size)
    (for _index_2 (range 1 _size)
      (bind _returnvalue (Game|SpawnActorfromClass "/Game/Blueprints/LifeCell.LifeCell_C" (Math|Transform|MakeTransform "0, 0, 0") "Undefined" 0 0))
      (CallFunction|AddCell _returnvalue)
      (Default|SetPositiononGrid _returnvalue _index_2 _index))))

(event EventTick
  (params (DeltaSeconds :type Float%20%28single-precision%29))
  (bind _returnvalue (Game|GetGameState))
  (bind _lifesimulatorcore (Variables|Default|GetLifeSimulatorCore))
  (bind _returnvalue_2 (GameState|GetServerWorldTimeSeconds _returnvalue))
  (if (Variables|LifeSimulator|GetSimulating)
    ;[1 1 1] Simulate the game of life
    (if (>= (- _returnvalue_2 (Variables|Utility|GetLastSimulation)) (Variables|LifeSimulator|GetSimulation%20Interval))
      (CallFunction|SimulationTick)
      (Variables|Utility|SetLastSimulation _returnvalue_2))
    (else
      ;[1 1 1] Cell activation/deactivation
      (bind _aslife_cell (Utilities|Casting|CastToLifeCell (.HitActor (Collision|BreakHitResult (.HitResult (Game|Player|GetHitResultUnderCursorbyChannel (Game|GetPlayerController 0) "TraceTypeQuery1" true))))))
      (switch Utilities|FlowControl|Switch|SwitchonLifeSimulator_ClickStatus (Variables|Utility|GetClickStatus)
        (:NewEnumerator1
          (Class|LifeSimulatorCore|SetCellValue _lifesimulatorcore (Variables|/Game/Blueprints/LifeCell.LifeCell_C|GetGrid%20X _aslife_cell) (Variables|/Game/Blueprints/LifeCell.LifeCell_C|GetGrid%20Y _aslife_cell) true))
        (:NewEnumerator2
          (Class|LifeSimulatorCore|SetCellValue _lifesimulatorcore (Variables|/Game/Blueprints/LifeCell.LifeCell_C|GetGrid%20X _aslife_cell) (Variables|/Game/Blueprints/LifeCell.LifeCell_C|GetGrid%20Y _aslife_cell) false)))
      (Default|UpdateMaterial _aslife_cell))))

(fn ConstructionScript)

(fn SimulationTick
  (Class|LifeSimulatorCore|CycleGrid (Variables|Default|GetLifeSimulatorCore))
  (for _array_element (Variables|LifeSimulator|GetCells)
    (Default|UpdateMaterial _array_element)))

(fn GetCellinPosition
  (params (Grid%20X :type Integer) (Grid%20Y :type Integer))
  (for _array_element (Variables|LifeSimulator|GetCells)
    (if (== (Variables|/Game/Blueprints/LifeCell.LifeCell_C|GetSimulator _array_element) self)
      (if (and (== (Variables|/Game/Blueprints/LifeCell.LifeCell_C|GetGrid%20X _array_element) Grid%20X) (== (Variables|/Game/Blueprints/LifeCell.LifeCell_C|GetGrid%20Y _array_element) Grid%20Y))
        (return _array_element))))
  (return 0))

(fn AddCell
  (params (Cell :type Life%20Cell%20Object%20Reference))
  (Variables|/Game/Blueprints/LifeCell.LifeCell_C|SetSimulator Cell self)
  (Utilities|Array|Add (Variables|LifeSimulator|GetCells) Cell))