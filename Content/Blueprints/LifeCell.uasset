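; LifeCell is an actor that displays one cell of a grid-based Life simulation owned by a Simulator.
; SetPositionOnGrid stores its coordinates and places it around the Simulator's location, using that grid's size and spacing to center the layout.
; UpdateMaterial reads the cell's value from LifeSimulatorCore, then toggles the point light and swaps between active and normal materials.
; Input is enabled at BeginPlay so cursor hover events can set the Highlighted flag.
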(event MouseInput|EventActorBeginCursorOver
  ;[1 1 1] Handle highlighting
  (Variables|Utility|SetHighlighted true))

(event MouseInput|EventActorEndCursorOver
  ;[1 1 1] Handle highlighting
  (Variables|Utility|SetHighlighted false))

(event EventBeginPlay
  ;[1 1 1] Enable input so we can highlight
  (Input|EnableInput (Game|GetPlayerController 0)))

(fn ConstructionScript)

(fn SetPositiononGrid
  (params (Grid%20X :type Integer) (Grid%20Y :type Integer))
  (bind _simulator (Variables|LifeCell|GetSimulator))
  (bind _size (Variables|/Game/Blueprints/LifeSimulator.LifeSimulator_C|GetSize _simulator))
  (bind _returnvalue (Math|Conversions|ToFloat(Integer) _size))
  (bind _returnvalue_2 (/ _returnvalue 2.0))
  (Variables|LifeCell|SetGrid%20X Grid%20X)
  (Variables|LifeCell|SetGrid%20Y Grid%20Y)
  (if (!= _simulator 0)
    (Transformation|SetActorLocation (+ (Transformation|GetActorLocation _simulator) (* (* (- (Math|Vector|MakeVector (- (Math|Conversions|ToFloat(Integer) Grid%20X) _returnvalue_2) (- (Math|Conversions|ToFloat(Integer) Grid%20Y) _returnvalue_2) 0.0) "-0.500000,0.500000,0.000000") "-1.000000,-1.000000,1.000000") (Variables|/Game/Blueprints/LifeSimulator.LifeSimulator_C|GetSpacing _simulator))) false true)))

(fn UpdateMaterial
  (bind _staticmeshcomponent (Variables|Debug|GetStaticMeshComponent))
  (bind _simulator (Variables|LifeCell|GetSimulator))
  (if (!= _simulator 0)
    (bind _returnvalue (Class|LifeSimulatorCore|GetCellValue (Variables|/Game/Blueprints/LifeSimulator.LifeSimulator_C|GetLifeSimulatorCore _simulator) (Variables|LifeCell|GetGrid%20X) (Variables|LifeCell|GetGrid%20Y)))
    (Rendering|SetVisibility (Variables|Default|GetPointLight) _returnvalue false)
    (if _returnvalue
      (Rendering|Material|SetMaterial _staticmeshcomponent 0 (Variables|LifeCell|GetActive%20Material))
      (else
        (Rendering|Material|SetMaterial _staticmeshcomponent 0 (Variables|LifeCell|GetNormal%20Material))))))