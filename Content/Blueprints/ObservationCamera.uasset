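; ObservationCamera is an orbit camera that lets the player rotate and zoom around a central root point.
; While the MoveCamera input is held, the mouse cursor hides and mouse delta rotates CameraRoot, with pitch clamped between angle limits.
; Zoom inputs step a clamped Distance, which Tick applies as the Camera's backward offset along local X whenever it differs.
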(event EventBeginPlay
  ;[1 1 1] Initialize distance
  (Variables|ObservationCamera|SetDistance (Variables|ObservationCamera|GetInitial%20Distance)))

(event EventTick
  (params (DeltaSeconds :type Float%20%28single-precision%29))
  (bind _returnvalue (Game|GetPlayerController 0))
  (bind _cameraroot (Variables|Default|GetCameraRoot))
  (bind _distance (Variables|ObservationCamera|GetDistance))
  (bind _camera (Variables|Default|GetCamera))
  (bind _returnvalue_2 (Transformation|GetRelativeTransform _cameraroot))
  (bind (_deltax _deltay) (Class|PlayerController|GetInputMouseDelta _returnvalue))
  (bind _returnvalue_3 (* _distance -1.0))
  (bind _rotation (Math|Transform|BreakTransform _returnvalue_2))
  (bind _returnvalue_4 (Math|Vector|MakeVector _returnvalue_3 0.0 0.0))
  (bind (_roll _pitch _yaw) (Math|Rotator|BreakRotator _rotation))
  (Utilities|FlowControl|Sequence
    (:then_0
      ;[1 1 1] Update camera distance
      (if (not (Math|Vector|Equal(Vector) (.Location (Math|Transform|BreakTransform (Transformation|GetRelativeTransform _camera))) _returnvalue_4 0.0001))
        (Transformation|SetRelativeLocation _camera _returnvalue_4 false false)))
    (:then_1
      ;[1 1 1] Handle camera movement
      (if (Variables|Utility|GetMoving)
        (Transformation|SetRelativeRotation _cameraroot (Math|Rotator|MakeRotator _roll (Math|Float|Clamp(Float) (+ _pitch (* _deltay (Variables|ObservationCamera|GetVertical%20Move%20Speed))) (Variables|ObservationCamera|GetMin%20Vertical%20Angle) (Variables|ObservationCamera|GetMax%20Vertical%20Angle)) (+ _yaw (* _deltax (Variables|ObservationCamera|GetHorizontal%20Move%20Speed)))) false false)))))

(event Input|ActionEvents|InputActionMoveCamera
  (params (Key :type Key%20Structure :default "AnyKey"))
  ;[1 1 1] Toggle camera movement
  (:Pressed
    (Variables|Utility|SetMoving true)
    (Variables|/Script/Engine.PlayerController|SetbShowMouseCursor (Game|GetPlayerController 0) (not (Variables|Utility|GetMoving)) :!label _label))
  (:Released
    (Variables|Utility|SetMoving false)
    (goto _label)))

(event Input|ActionEvents|InputActionMoveCameraCloser
  (params (Key :type Key%20Structure :default "AnyKey"))
  ;[1 1 1] Change camera zoom
  (:Pressed
    (Variables|ObservationCamera|SetDistance (Math|Float|Clamp(Float) (- (Variables|ObservationCamera|GetDistance) (Variables|ObservationCamera|GetDistance%20Change%20Interval)) (Variables|ObservationCamera|GetMin%20Distance) (Variables|ObservationCamera|GetMax%20Distance)))))

(event Input|ActionEvents|InputActionMoveCameraFurther
  (params (Key :type Key%20Structure :default "AnyKey"))
  ;[1 1 1] Change camera zoom
  (:Pressed
    (Variables|ObservationCamera|SetDistance (Math|Float|Clamp(Float) (+ (Variables|ObservationCamera|GetDistance) (Variables|ObservationCamera|GetDistance%20Change%20Interval)) (Variables|ObservationCamera|GetMin%20Distance) (Variables|ObservationCamera|GetMax%20Distance)))))

(fn ConstructionScript)